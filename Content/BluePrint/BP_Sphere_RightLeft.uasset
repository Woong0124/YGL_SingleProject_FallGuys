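; BP_Sphere_RightLeft is a moving sphere hazard that rolls back and forth sideways and ragdolls any BP_Character it hits.
; A timeline scaled by EndPoint drives the sphere's relative Y location, alternating between Play and Reverse by toggling IsRight on each finish.
; Each update also adds a fixed local rotation, with its sign flipped by IsReverse so the spin follows the travel direction.
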(event `self.ReceiveHit`
  (params (MyComp :type "PrimitiveComponent Object Reference") (Other :type "Actor Object Reference") (OtherComp :type "PrimitiveComponent Object Reference") (bSelfMoved :type Boolean) (HitLocation :type "Vector Structure") (HitNormal :type "Vector Structure") (NormalImpulse :type "Vector Structure") (Hit :type "HitResult Structure (by ref)"))
  (bind _asbp_character (cast `/Game/BluePrint/BP_Character` Other))
  (`/Game/BluePrint/BP_Character.DoRagDoll` _asbp_character))

(event `self.ReceiveBeginPlay`
  (if (`self.IsRight`) :!label _label
    (set `self.IsReverse` false)
    (bind (_direction _rightleft) (`Timeline|RIghtLeft` :!label _label_2)
      (:`Update`
        (`SceneComponent.K2_SetRelativeLocation` (`self.Sphere`) (`KismetMathLibrary.MakeVector` 0.0 (* _rightleft (`self.EndPoint`))) false false)
        ;[1 1 1] 정방향인지 아닌지에 따라 공 회전 변경
        (if (== (`self.IsReverse`) false)
          (`SceneComponent.K2_AddLocalRotation` (`self.Sphere`) (struct :`Roll` 3.5) false false)
          (else
            (`SceneComponent.K2_AddLocalRotation` (`self.Sphere`) (struct :`Roll` -3.5) false false))))
      (:`Finished`
        (set `self.IsRight` (not (`self.IsRight`)))
        (goto _label)))
    (else
      (set `self.IsReverse` true)
      (goto _label_2 :!via `Reverse`))))

(fn `UserConstructionScript`)