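; BP_Sphere_Weight is a swinging weight obstacle that sends BP_Character into ragdoll on hit.
; Tick rolls the root component by SetRotate each frame and advances a separate counter, AddRotate, without delta time scaling.
; When the counter reaches EndPoint, it resets and passes through two toggled Gates that set SetRotate's sign to reverse the swing.
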(event `self.ReceiveTick`
  (params (DeltaSeconds :type "Float (single-precision)"))
  (bind _returnvalue (+ (`self.AddRotate`) 1.5))
  ;[1 1 1] 엑터 회전
  (`SceneComponent.K2_AddRelativeRotation` (`self.DefaultSceneRoot`) (`KismetMathLibrary.MakeRotator` (`self.SetRotate`)) false false)
  ;[1 1 1] 180도를 돌았는지 확인
  (set `self.AddRotate` _returnvalue)
  (if (>= _returnvalue (`self.EndPoint`))
    ;[1 1 1] 얼마나 회전했는지 값 초기화
    (set `self.AddRotate` 0.0)
    ;[1 1 1] 회전값 설정
    (`|ExecutionSequence`
      (:`then_0`
        (`/Engine/EditorBlueprintResources/StandardMacros.Gate` false :!label _label
          (:`Exit`
            (set `self.SetRotate` -1.3))))
      (:`then_1`
        (`/Engine/EditorBlueprintResources/StandardMacros.Gate` true :!label _label_2
          (:`Exit`
            (set `self.SetRotate` 1.3))))
      (:`then_2`
        (goto _label :!via `Toggle`))
      (:`then_3`
        (goto _label_2 :!via `Toggle`)))))

(event `self.ReceiveHit`
  (params (MyComp :type "PrimitiveComponent Object Reference") (Other :type "Actor Object Reference") (OtherComp :type "PrimitiveComponent Object Reference") (bSelfMoved :type Boolean) (HitLocation :type "Vector Structure") (HitNormal :type "Vector Structure") (NormalImpulse :type "Vector Structure") (Hit :type "HitResult Structure (by ref)"))
  (bind _asbp_character (cast `/Game/BluePrint/BP_Character` Other))
  (`/Game/BluePrint/BP_Character.DoRagDoll` _asbp_character))

(fn `UserConstructionScript`)