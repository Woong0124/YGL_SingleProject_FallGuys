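; BP_Cube_Box is a gold box collectible that keeps relocating around the level until the player has collected ten.
; It binds Hit to BP_Character's gold box event, which spawns a replacement, plays effects, increments GoldBoxCount and destroys itself.
; A gated Tick destroys the box at ten, and a delay otherwise respawns it at a random position.
; Relocation works by spawning a new copy rather than moving the actor.
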(event `self.ReceiveTick`
  (params (DeltaSeconds :type "Float (single-precision)"))
  ;[1 1 1] 골드박스를 10개 모았으면 더이상 스폰 X
  (`/Engine/EditorBlueprintResources/StandardMacros.Gate` false :!label _label
    (:`Exit`
      (`|ExecutionSequence`
        (:`then_0`
          (bind _asbp_character (cast `/Game/BluePrint/BP_Character` (`GameplayStatics.GetPlayerCharacter` 0)))
          (if (>= (`/Game/BluePrint/BP_Character.GoldBoxCount` _asbp_character) 10)
            (`self.K2_DestroyActor`)
            (goto _label :!via `Close`)))
        (:`then_1`
          ;[1 1 1] 일정 시간 지난뒤 랜덤 지역 이동
          (`KismetSystemLibrary.Delay` 4.5)
          (`|SpawnActorFromClass` "BP_Cube_Box_C" (`KismetMathLibrary.MakeTransform` (`KismetMathLibrary.MakeVector` (`KismetMathLibrary.RandomFloatInRange` -1200.0 1200.0) (`KismetMathLibrary.RandomFloatInRange` -1200.0 1200.0) 71.0)) "Undefined" "OverrideRootScale" null null)
          (`self.K2_DestroyActor`))))))

(event `self.ReceiveBeginPlay`
  ;[1 1 1] 시작 시 골드박스 획득 이벤트 바인딩
  (bind _asbp_character (cast `/Game/BluePrint/BP_Character` (`GameplayStatics.GetPlayerCharacter` 0)))
  (add `/Game/BluePrint/BP_Character.GetGoldBox` _asbp_character (delegate `Hit`)))

(event `Hit`
  (bind _returnvalue (`SceneComponent.K2_GetComponentLocation` (`self.Cube`)))
  ;[1 1 1] 캐릭터가 골드 박스를 획득 했다면 실행 ( 새로 스폰, 캐릭터 GoldBoxCount 1씩 증가, 자기 자신 파괴 )
  (`|SpawnActorFromClass` "BP_Cube_Box_C" (`KismetMathLibrary.MakeTransform` (`KismetMathLibrary.MakeVector` (`KismetMathLibrary.RandomFloatInRange` -1300.0 1300.0) (`KismetMathLibrary.RandomFloatInRange` -1300.0 1300.0) 71.0)) "Undefined" "OverrideRootScale" null null)
  (`GameplayStatics.SpawnSoundAtLocation` "/Game/Sound/SC_CheakPoint.SC_CheakPoint" _returnvalue (struct) 1.0 1.0 0.0 null null)
  (`GameplayStatics.SpawnEmitterAtLocation` "/Game/Realistic_Starter_VFX_Pack_Vol2/Particles/Destruction/P_Destruction_Metal.P_Destruction_Metal" _returnvalue)
  (bind _asbp_character (cast `/Game/BluePrint/BP_Character` (`GameplayStatics.GetPlayerCharacter` 0)))
  (bind _result (`/Engine/EditorBlueprintResources/StandardMacros.IncrementInt` (`/Game/BluePrint/BP_Character.GoldBoxCount` _asbp_character))
    (:`  `
      (set `/Game/BluePrint/BP_Character.GoldBoxCount` _result _asbp_character)
      (`self.K2_DestroyActor`))))

(fn `UserConstructionScript`)