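; Blueprint actor whose Cube component moves continuously up and down within a height range.
; Tick adds a fixed relative Z offset each frame without sweep, so speed depends on frame rate.
; The IsMoveUp flag sets direction, flipping when relative Z passes the EndPoint variable at the top or reaches a hardcoded lower limit.
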(event `self.ReceiveTick`
  (params (DeltaSeconds :type "Float (single-precision)"))
  (bind _cube (`self.Cube`))
  (bind (_relativelocation_x _relativelocation_y _relativelocation_z) (`KismetMathLibrary.BreakVector` (`SceneComponent.RelativeLocation` _cube)))
  ;[1 1 1] 큐브가 위, 아래로 범위내에서 이동
  (if (`self.IsMoveUp`)
    (`SceneComponent.K2_AddRelativeLocation` _cube (0.0 0.0 2.0) false false)
    (if (> _relativelocation_z (`self.EndPoint`))
      (set `self.IsMoveUp` false))
    (else
      (`SceneComponent.K2_AddRelativeLocation` _cube (0.0 0.0 -2.0) false false)
      (if (<= _relativelocation_z 140.0)
        (set `self.IsMoveUp` true)))))

(fn `UserConstructionScript`)