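; Player character Blueprint with camera-relative movement, jumping, an F-held montage chosen from BP_Instance, and gold box collection.
; Hitting the BP_Cube_Box actor fires the GetGoldBox dispatcher while the count is below ten.
; DoRagDoll simulates mesh physics with the actor following, then a timed DoGetUp reattaches the mesh.
; Tick then teleports to SetLocation and adds audio, and also halts movement during the F and cheering montages.
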(event `InputAxis|Move_Foward`
  (params (AxisValue :type "Float (single-precision)"))
  ;[1 1 1] 캐릭터 이동
  (`self.AddMovementInput` (`KismetMathLibrary.GetForwardVector` (`KismetMathLibrary.MakeRotator` 0.0 0.0 (.yaw (`self.GetControlRotation`)))) AxisValue))

(event `InputAxis|Turn`
  (params (AxisValue :type "Float (single-precision)"))
  ;[1 1 1] 마우스 이동
  (`self.AddControllerYawInput` AxisValue))

(event `InputAxis|Move_Right`
  (params (AxisValue :type "Float (single-precision)"))
  ;[1 1 1] 캐릭터 이동
  (`self.AddMovementInput` (`KismetMathLibrary.GetRightVector` (`KismetMathLibrary.MakeRotator` 0.0 0.0 (.yaw (`self.GetControlRotation`)))) AxisValue))

(event `InputAxis|Look_Up`
  (params (AxisValue :type "Float (single-precision)"))
  ;[1 1 1] 마우스 이동
  (`self.AddControllerPitchInput` AxisValue))

(event `self.ReceiveTick`
  (params (DeltaSeconds :type "Float (single-precision)"))
  (`|ExecutionSequence`
    (:`then_0`
      ;[1 1 1] Ragdoll 중일 때 위치 설정
      (if (`self.IsRagDoll`)
        (`self.K2_SetActorLocation` (`SceneComponent.K2_GetComponentLocation` (`self.Mesh`)))))
    (:`then_1`
      ;[1 1 1] Ragdoll이 끝나면 타깃포인트의 위치로 스폰과 함께 몽타주 실행
      (if (`self.RagDollFin`)
        (`SceneComponent.K2_SetWorldRotation` (`self.CapsuleComponent`) (struct :`Yaw` 180.0) false false)
        (`self.K2_SetActorLocation` (`self.SetLocation`))
        (set `self.RagDollFin` false)
        (`AddComponent|NODE_AddAudioComponent-0`)))
    (:`then_2`
      (`|ExecutionSequence`
        (:`then_0`
          ;[1 1 1] 겟업 몽타주 중에 움직임 X
          (if (`AnimInstance.Montage_IsPlaying` (`SkeletalMeshComponent.GetAnimInstance` (`self.Mesh`)) "/Game/Character/Cheering_Montage.Cheering_Montage")
            (`MovementComponent.StopMovementImmediately` (`self.CharacterMovement`))))
        (:`then_1`
          ;[1 1 1] f 몽타주 중에 움직임 X
          (if (`AnimInstance.Montage_IsPlaying` (`SkeletalMeshComponent.GetAnimInstance` (`self.Mesh`)) (`self.Montage`))
            (`MovementComponent.StopMovementImmediately` (`self.CharacterMovement`))))))))

(event `Key|SpaceBar`
  (params (Key :type "Key Structure"))
  ;[1 1 1] 점프
  (:`Pressed`
    (`self.Jump`)))

(event `self.ReceiveHit`
  (params (MyComp :type "PrimitiveComponent Object Reference") (Other :type "Actor Object Reference") (OtherComp :type "PrimitiveComponent Object Reference") (bSelfMoved :type Boolean) (HitLocation :type "Vector Structure") (HitNormal :type "Vector Structure") (NormalImpulse :type "Vector Structure") (Hit :type "HitResult Structure (by ref)"))
  ;[1 1 1] 캐릭터와 골드박스가 충돌 했을 때 이벤트디스패처 호출
  (bind _returnvalue (`GameplayStatics.GetActorOfClass` "/Game/BluePrint/BP_Cube_Box.BP_Cube_Box_C"))
  (if (== _returnvalue Other)
    (if (not (>= (`self.GoldBoxCount`) 10))
      ;;[1 0 0] Cube_Box, UMG_Start 에 바인딩 됨
      (`self.GetGoldBox`))))

(event `Key|F`
  (params (Key :type "Key Structure"))
  (bind _montage (`self.Montage`))
  ;[1 1 1] F키 모션 몽타주
  (:`Pressed`
    (bind _asbp_instance (cast `/Game/BluePrint/BP_Instance` (`GameplayStatics.GetGameInstance`)))
    (set `self.Montage` (`/Game/BluePrint/BP_Instance.IMontage` _asbp_instance))
    (if (not (`NavMovementComponent.IsFalling` (`self.CharacterMovement`)))
      (`self.PlayAnimMontage` _montage)))
  (:`Released`
    (`self.StopAnimMontage` _montage)))

(fn `DoGetUp`
  (set `self.IsRagDoll` false)
  (`PrimitiveComponent.SetSimulatePhysics` (`self.Mesh`) false)
  (`SceneComponent.K2_AttachToComponent` (`self.Mesh`) (`self.CapsuleComponent`) "None" "KeepRelative" "KeepRelative" "KeepRelative" true)
  (`SceneComponent.K2_SetRelativeLocationAndRotation` (`self.Mesh`) (0.0 0.0 -89.0) (struct :`Yaw` -90.0) false false)
  (set `self.RagDollFin` true))

(fn `DoRagDoll`
  (set `self.IsRagDoll` true)
  (`PrimitiveComponent.SetSimulatePhysics` (`self.Mesh`) true)
  (`KismetSystemLibrary.K2_SetTimer` null "DoGetUp" 2.5))

(fn `UserConstructionScript`)